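; Cartman character Blueprint that animates a 2D mouth sprite and a blink morph target from lip-sync and Live Link data.
; Each Tick evaluates a Live Link Basic role frame; on a valid frame, the strongest OVR LipSync playback viseme selects the mouth sprite.
; On the invalid-frame branch, ARKit property values from that evaluation drive BLINK and toggle between two mouth sprites by a threshold.
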(event EventBeginPlay)

(event Collision|EventActorBeginOverlap
  (params (OtherActor :type Actor%20Object%20Reference)))

(event EventTick
  (params (DeltaSeconds :type Float%20%28single-precision%29))
  (bind _ovrlipsyncplaybackactor (Variables|Default|GetOVRLipSyncPlaybackActor))
  (bind _dataresult (|EvaluateLiveLinkFramewithSpecificRole "(Name=\"Python_LiveLinkFace\")" "/Script/LiveLinkInterface.LiveLinkBasicRole")
    (:then
      (Variables|Default|SetViseme_Names (Class|OVRLipSyncActorComponentBase|GetVisemeNames _ovrlipsyncplaybackactor))
      (bind _output_get (Variables|Default|SetViseme_Values (Class|OVRLipSyncActorComponentBase|GetVisemes _ovrlipsyncplaybackactor)))
      (for (_array_element _array_index) _output_get
        (if (> _array_element (Variables|Default|GetHighestValViseme))
          (Variables|Default|SetHighestValViseme _array_element)
          (Variables|Default|SetIndex _array_index)))
      (Rendering|Components|Sprite|SetSprite (Variables|Default|GetPaperSprite) (Utilities|Array|Get(acopy) (Variables|Default|GetVisemeSprites) (Variables|Default|GetIndex)))
      (Variables|Default|SetHighestValViseme 0.0))
    (:InvalidFrame
      (Variables|Default|SetARkitNames (Utilities|Struct|BreakLiveLinkBaseStaticData (.StaticData (Utilities|Struct|BreakLiveLinkBasicBlueprintData _dataresult))))
      (bind _output_get_2 (Variables|Default|SetARkit%20Values (.PropertyValues (Utilities|Struct|BreakLiveLinkBaseFrameData (.FrameData (Utilities|Struct|BreakLiveLinkBasicBlueprintData _dataresult))))))
      (Components|SkeletalMesh|SetMorphTarget (Variables|Default|GetCharacter) "BLINK" (Math|Conversions|ToFloat(Integer) (Utilities|String|ToString(Float) (Utilities|Array|Get(acopy) _output_get_2))) true)
      (if (> (Utilities|Array|Get(acopy) _output_get_2 17) 0.5)
        (Rendering|Components|Sprite|SetSprite (Variables|Default|GetPaperSprite) "/Game/2D_Visemes/kisspng-drawing-black-and-white-art-lip-sync-animations-vector-5adb9d7c225d55_5811137315243421401408_Sprite_14.kisspng-drawing-black-and-white-art-lip-sync-animations-vector-5adb9d7c225d55_5811137315243421401408_Sprite_14")
        (else
          (Rendering|Components|Sprite|SetSprite (Variables|Default|GetPaperSprite) "/Game/2D_Visemes/kisspng-drawing-black-and-white-art-lip-sync-animations-vector-5adb9d7c225d55_5811137315243421401408_Sprite_4.kisspng-drawing-black-and-white-art-lip-sync-animations-vector-5adb9d7c225d55_5811137315243421401408_Sprite_4"))))))

(fn ConstructionScript)