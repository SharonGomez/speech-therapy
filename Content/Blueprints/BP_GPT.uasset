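; BP_GPT is a prototype actor that requests an AI-generated image from a text Prompt and shows it on its Frame mesh.
; The generate event requests Base64 JSON image data, converts it and caches the result as PromptImage.
; A separate update event applies PromptImage to the frame's dynamic material and draws that material to a render target.
; SaveImage is an empty stub, and debug prints and TODO placeholders remain throughout.
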(event Custom|Generate%20Image
  (Development|PrintString "Calling FUNCTION" true true "(R=0.234375,G=0.093516,B=0.000000,A=1.000000)" 1e+01)
  (bind _response (|RequestImagesCustomOptions :Prompt (Variables|Default|GetPrompt) :ImageOptions (Utilities|Struct|MakeHttpGPTImageOptions 1 "x256" "b64_json"))
    (:then
      (Class|HttpGPTImageHelper|GenerateImage (Utilities|Array|Get(acopy) (.data _response)) (delegate Custom|Image2Frame)))
    (:ErrorReceived
      (Development|PrintString "ERROR" true true "(R=1.000000,G=0.076389,B=0.076389,A=1.000000)" 1e+01 :!label _label))
    (:RequestFailed
      (goto _label))))

(event Custom|Image2Frame
  (params (Image :type Texture%202D%20Object%20Reference))
  ;[1 1 1] Delegate
  (Variables|Default|SetPrompt%20Image Image)
  (Development|PrintString "IMAGE GENERATED FINAL" true true "(R=0.000000,G=0.660000,B=1.000000,A=1.000000)" 1e+01))

(event Custom|Update%20Frame
  (Rendering|Material|SetTextureParameterValue (Variables|Default|GetDynamic%20Material%20Image) "PromptImage" (Variables|Default|GetPrompt%20Image))
  (Rendering|DrawMaterialtoRenderTarget (Variables|Default|GetTexture%20Render%20Target) (Variables|Default|GetDynamic%20Material%20Image)))

(event Custom|Save%20Image)

(event Custom|event_gen
  (Development|PrintString "Generate Image Pressed")
  (Utilities|FlowControl|Sequence
    (:then_0
      (CallFunction|GenerateImage)
      ;[1 0.3212 0.3212] TODO
      (Development|PrintString "To do")
      (Utilities|FlowControl|Delay 1e+01)
      ;[1 0.3212 0.3212] TODO
      (Development|PrintString "To do"))
    (:then_1
      (Utilities|FlowControl|DoOnce false ; enters at Reset
        (:Completed
          (CallFunction|SaveImage)
          ;[1 0.3212 0.3212] TODO
          (Development|PrintString "To do")
          ;[1 0.3212 0.3212] TODO
          (Development|PrintString "To do"))))))

(event Custom|event_update
  (Development|PrintString "Update Image Pressed")
  (CallFunction|UpdateFrame)
  ;[1 0.3212 0.3212] TODO
  (Development|PrintString "To do")
  ;[1 0.3212 0.3212] TODO
  (Development|PrintString "To do"))

(event EventBeginPlay
  (Utilities|FlowControl|Sequence
    (:then_1
      (bind _returnvalue (Rendering|Material|CreateDynamicMaterialInstance (Variables|Default|GetFrame) 1 "/Game/Materials/M_GPT_Inst.M_GPT_Inst" "None" :!class /Script/Engine.PrimitiveComponent))
      (Variables|Default|SetDynamic%20Material%20Image _returnvalue)
      (Development|PrintString "Hello" true true "(R=0.185764,G=0.118491,B=0.016371,A=1.000000)"))))

(event Input|KeyboardEvents|F9
  (params (Key :type Key%20Structure :default "None"))
  ;[1 1 1] Comment
)

(fn ConstructionScript)