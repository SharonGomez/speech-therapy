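; Actor Blueprint that experiments with OpenAI chat requests through an OpenAI plugin.
; A chain headed by SetOpenAIApiKey sends a GPT-3.5 Turbo chat call, then prints the response's finish reason, rather than its text, or the error message on failure.
; The AskAi event holds only an empty model switch, and BeginPlay, overlap, Tick and the construction script do nothing.
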(event Custom|Ask%20Ai_1_1
  (switch Utilities|FlowControl|Switch|SwitchonEHttpGPTChatModel "gpt35turbo"))

(event EventBeginPlay)

(event Collision|EventActorBeginOverlap
  (params (OtherActor :type Actor%20Object%20Reference)))

(event EventTick
  (params (DeltaSeconds :type Float%20%28single-precision%29)))

(fn ConstructionScript)